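; Placeable ambient sound Blueprint that plays a configurable SoundCue when a qualifying actor enters its sphere trigger.
; The construction script applies the cue, attenuation settings and trigger radius to the components.
; Overlapping actors that pass an interface check trigger playback through events named for the owning client, optionally at a random start time.
; A DoOnce gate prevents repeat triggers until any end overlap resets it, without stopping the audio.
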(event OnComponentBeginOverlap(SphereRadi)
  (params (OverlappedComponent :type Primitive%20Component%20Object%20Reference) (OtherActor :type Actor%20Object%20Reference) (OtherComp :type Primitive%20Component%20Object%20Reference) (OtherBodyIndex :type Integer) (bFromSweep :type Boolean) (SweepResult :type Hit%20Result%20Structure%20%28by%20ref%29))
  (if (Utilities|DoesObjectImplementInterface OtherActor 0)
    (CallFunction|SendAudioPlayCommandOwningClient (Variables|Default|GetAmbientAudio) (Variables|Default|GetSoundCue))))

(event OnComponentEndOverlap(SphereRadi)
  (params (OverlappedComponent :type Primitive%20Component%20Object%20Reference) (OtherActor :type Actor%20Object%20Reference) (OtherComp :type Primitive%20Component%20Object%20Reference) (OtherBodyIndex :type Integer))
  (Utilities|FlowControl|DoOnce false) ; enters at Reset
)

(event Custom|SendAudioPlayCommandOwningClient
  (params (AmbientAudioComponent :type Audio%20Component%20Object%20Reference) (SoundCue :type Sound%20Base%20Object%20Reference))
  (Utilities|FlowControl|DoOnce false
    (:Completed
      (CallFunction|RunAudioonOwningClient AmbientAudioComponent SoundCue))))

(event Custom|RunAudioOnOwningClient
  (params (AmbientAudioComponent :type Audio%20Component%20Object%20Reference) (SoundCue :type Sound%20Base%20Object%20Reference))
  (Audio|Components|Audio|Play AmbientAudioComponent (Math|Float|SelectFloat (Math|Random|RandomFloatinRange 0.0 (Variables|/Script/Engine.SoundBase|GetDuration SoundCue)) 0.0 (Variables|Default|Getstarttimerandom))))

(event Collision|EventActorBeginOverlap
  (params (OtherActor :type Actor%20Object%20Reference)))

(event EventTick
  (params (DeltaSeconds :type Float%20%28single-precision%29)))

(event EventBeginPlay)

(fn ConstructionScript
  (Audio|Components|Audio|SetSound (Variables|Default|GetAmbientAudio) (Variables|Default|GetSoundCue))
  (Variables|/Script/Engine.AudioComponent|SetAttenuationSettings (Variables|Default|GetAmbientAudio) (Variables|Default|GetAmbientSoundAttenuation))
  (Components|Sphere|SetSphereRadius (Variables|Default|GetSphereRadi) (Variables|Default|GetRadius) true))